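; Player character for a twin-stick arena shooter that moves, aims, fires and takes damage from enemies.
; BeginPlay spawns an ArenaWeaponBP and attaches it to the mesh's GunSocket.
; Move axes drive world-space movement, while both look axes share logic that sets control rotation and starts firing past a deadzone, stopping otherwise.
; Hits from Enemy-tagged actors reduce Health, destroying the character when it runs out.
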(event `Take Damage`
  (bind _output_get (set `self.Health` (- (`self.Health`) 10)))
  (if (<= _output_get 0)
    (`self.K2_DestroyActor`)))

(event `self.ReceiveHit`
  (params (MyComp :type "PrimitiveComponent Object Reference") (Other :type "Actor Object Reference") (OtherComp :type "PrimitiveComponent Object Reference") (bSelfMoved :type Boolean) (HitLocation :type "Vector Structure") (HitNormal :type "Vector Structure") (NormalImpulse :type "Vector Structure") (Hit :type "HitResult Structure (by ref)"))
  (if (`self.ActorHasTag` Other "Enemy")
    (`self.Take Damage`)))

(event `self.ReceiveBeginPlay`
  (bind _returnvalue (`|SpawnActorFromClass` "/Game/Blueprints/ArenaWeaponBP.ArenaWeaponBP_C" (`SceneComponent.K2_GetComponentToWorld` (`self.Mesh`)) "Undefined" "OverrideRootScale" null null))
  (bind _output_get (set `self.Weapon` _returnvalue))
  (`self.K2_AttachToComponent` _output_get (`self.Mesh`) "GunSocket" "SnapToTarget" "SnapToTarget" "SnapToTarget" false))

(event `InputAxis|MoveUp`
  (params (AxisValue :type "Float (single-precision)"))
  ;[1 1 1] Character Movement
  (`self.AddMovementInput` (1.0 0.0 0.0) AxisValue))

(event `InputAxis|LookUp`
  (params (AxisValue :type "Float (single-precision)"))
  ;[1 1 1] Character Movement
  (bind _returnvalue (`KismetMathLibrary.MakeVector` AxisValue (stale `InputAxis|LookRight` AxisValue)))
  (if (> (`KismetMathLibrary.VSize` _returnvalue) 0.5) :!label _label
    (`Controller.SetControlRotation` (`GameplayStatics.GetPlayerController` 0) (`KismetMathLibrary.MakeRotFromX` _returnvalue))
    (`/Game/Blueprints/ArenaWeaponBP.StartFire` (`self.Weapon`))
    (else
      (`/Game/Blueprints/ArenaWeaponBP.StopFire` (`self.Weapon`)))))

(event `InputAxis|MoveRight`
  (params (AxisValue :type "Float (single-precision)"))
  ;[1 1 1] Character Movement
  (`self.AddMovementInput` (0.0 1.0 0.0) AxisValue))

(event `InputAxis|LookRight`
  (params (AxisValue :type "Float (single-precision)"))
  ;[1 1 1] Character Movement
  (goto _label))

(fn `UserConstructionScript`)