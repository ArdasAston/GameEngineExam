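; ArenaWeaponBP is an arena weapon that fires projectiles automatically between start and stop fire events.
; StartFire passes a DoOnce gate, fires immediately, then starts a looping timer that repeats Fire at the FireRate interval.
; Each shot spawns an ArenaProjectileBP at the Gun component's world transform.
; StopFire clears the timer and resets the gate, so repeated start calls cannot stack timers.
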(event `StartFire`
  (`/Engine/EditorBlueprintResources/StandardMacros.DoOnce` false :!label _label
    (:`Completed`
      (`self.Fire`)
      (bind _returnvalue (`KismetSystemLibrary.K2_SetTimerDelegate` (delegate `Fire`) (`self.FireRate`) true))
      (set `self.FireTimer` _returnvalue))))

(event `StopFire`
  (`KismetSystemLibrary.K2_ClearAndInvalidateTimerHandle` (`self.FireTimer`))
  (goto _label :!via `Reset`))

(event `Fire`
  (`|SpawnActorFromClass` "/Game/Blueprints/ArenaProjectileBP.ArenaProjectileBP_C" (`SceneComponent.K2_GetComponentToWorld` (`self.Gun`)) "Undefined" "OverrideRootScale" null null))

(fn `UserConstructionScript`)