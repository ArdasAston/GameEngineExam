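; ArenaEnemyBP is an arena enemy that takes damage and reports its death to the game mode.
; Each Die event removes a fixed amount of Health, so it acts as a hit rather than an instant kill.
; At zero Health or below it destroys itself, then calls DecreaseEnemies on ArenaGameModeBP.
; The construction script creates a dynamic material instance of Mat_Enemy on the mesh.
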(event `Die`
  (bind _output_get (set `self.Health` (- (`self.Health`) 10)))
  (if (<= _output_get 0)
    (`self.K2_DestroyActor`)
    (bind _asarena_game_mode_bp (cast `/Game/Blueprints/ArenaGameModeBP` (`GameplayStatics.GetGameMode`)))
    (`/Game/Blueprints/ArenaGameModeBP.Decrease Enemies` _asarena_game_mode_bp)))

(fn `UserConstructionScript`
  (`PrimitiveComponent.CreateDynamicMaterialInstance` (`self.Mesh`) 0 "/Game/Materials/Mat_Enemy.Mat_Enemy" "None"))