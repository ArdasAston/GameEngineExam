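; EnemySpawnerBP is an arena enemy spawner that, when Active at BeginPlay, repeatedly spawns batches of the configured enemy class at its own transform.
; SpawnEnemy spawns a batch, waits SpawnDelay, then calls itself while ArenaGameModeBP's enemy count is below its maximum.
; At the cap, ShouldSpawn polls on the same delay until room opens.
; IncreaseEnemies runs on the game mode once per batch, regardless of batch size.
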(event `self.ReceiveBeginPlay`
  (`|ExecutionSequence`
    (:`then_0`
      (if (`self.Active?`)
        (`self.Spawn Enemy` (`self.Enemy`) (`self.GetTransform`) (`self.Number Of Enemy`))
        (bind _asarena_game_mode_bp (cast `/Game/Blueprints/ArenaGameModeBP` (`GameplayStatics.GetGameMode`)))
        (`/Game/Blueprints/ArenaGameModeBP.Increase Enemies` _asarena_game_mode_bp)))
    (:`then_1`
      (bind _asarena_game_mode_bp_2 (cast `/Game/Blueprints/ArenaGameModeBP` (`GameplayStatics.GetGameMode`)))
      (set `self.Arena Game Mode Ref` _asarena_game_mode_bp_2))))

(event `Spawn Enemy`
  (params (Enemy :type "Actor Class Reference") (SpawnTransform :type "Transform Structure") (`Number Of Enemy` :type Integer))
  (bind _arena_game_mode_ref (`self.Arena Game Mode Ref`))
  (for _ (range `Number Of Enemy`)
    (`|SpawnActorFromClass` Enemy SpawnTransform "Undefined" "OverrideRootScale" null null))
  (`KismetSystemLibrary.Delay` (`self.Spawn Delay`))
  (if (< (`/Game/Blueprints/ArenaGameModeBP.Enemies In Level` _arena_game_mode_ref) (`/Game/Blueprints/ArenaGameModeBP.Max Enemies` _arena_game_mode_ref))
    (`self.Spawn Enemy` (`self.Enemy`) (`self.GetTransform`) (`self.Number Of Enemy`))
    (bind _asarena_game_mode_bp (cast `/Game/Blueprints/ArenaGameModeBP` (`GameplayStatics.GetGameMode`)))
    (`/Game/Blueprints/ArenaGameModeBP.Increase Enemies` _asarena_game_mode_bp)
    (else
      (`self.ShouldSpawn?`))))

(event `ShouldSpawn?`
  (bind _arena_game_mode_ref (`self.Arena Game Mode Ref`))
  (`KismetSystemLibrary.Delay` (`self.Spawn Delay`))
  (if (< (`/Game/Blueprints/ArenaGameModeBP.Enemies In Level` _arena_game_mode_ref) (`/Game/Blueprints/ArenaGameModeBP.Max Enemies` _arena_game_mode_ref))
    (`self.Spawn Enemy` (`self.Enemy`) (`self.GetTransform`) (`self.Number Of Enemy`))
    (bind _asarena_game_mode_bp (cast `/Game/Blueprints/ArenaGameModeBP` (`GameplayStatics.GetGameMode`)))
    (`/Game/Blueprints/ArenaGameModeBP.Increase Enemies` _asarena_game_mode_bp)
    (else
      (`self.ShouldSpawn?`))))

(fn `UserConstructionScript`)